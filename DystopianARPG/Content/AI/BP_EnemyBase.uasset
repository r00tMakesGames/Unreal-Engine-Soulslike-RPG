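; Base enemy AI Blueprint that roams around its spawn point, then chases and melees an assigned player target.
; Roaming repeats AIMoveTo to random reachable points until SetPlayerTarget switches it to running combat, with Tick yawing it toward the player.
; A distant target triggers a taunt before a chase-and-attack loop timed by random montage lengths.
; MeleeSphere collision is switchable by event, and ClearTarget is an empty stub.
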(event Custom|play%20montage
  (params (InSkeletalMeshComponent :type Skeletal%20Mesh%20Component%20Object%20Reference) (MontageToPlay :type Anim%20Montage%20Object%20Reference) (StartingSection :type Name))
  (Animation|Montage|PlayMontage InSkeletalMeshComponent MontageToPlay 1.0 0.0 StartingSection))

(event EventBeginPlay
  ;[1 1 1] Begin Play
  (CallFunction|FMovementState "NewEnumerator1")
  (Variables|Default|SetStartingLocation (Transformation|GetActorLocation))
  (Utilities|FlowControl|Delay 1.0)
  (CallFunction|SetRoaming))

(event Collision|EventActorBeginOverlap
  (params (OtherActor :type Actor%20Object%20Reference))
  ;[1 1 1] Begin Play
)

(event EventRunAttacks
  (Variables|Default|GetPlayerTarget
    (:then
      (bind _length (CallFunction|FPickAttack (Transformation|GetDistanceTo self (Variables|Default|GetPlayerTarget))))
      (Utilities|FlowControl|Delay (+ _length 0.5))
      (CallFunction|ChasePlayer))
    (:else
      (CallFunction|ClearTarget))))

(event EventSetRoaming
  ;[1 1 1] Roaming
  (if (and (not (Variables|Default|GetIsRoaming)) (not (Variables|Default|GetIsCombat)))
    (AI|AIMoveTo self (.RandomLocation (AI|Navigation|GetRandomReachablePointinRadius (Variables|Default|GetStartingLocation) 5e+04 0 0)) 0 7e+01 false
      (:then
        (Variables|Default|SetIsRoaming true))
      (:OnSuccess
        (Variables|Default|SetIsRoaming false)
        (Utilities|FlowControl|Delay 2.0)
        (CallFunction|SetRoaming)))))

(event EventSetPlayerTarget
  (params (Target :type Actor%20Object%20Reference))
  ;[1 1 1] Set Player Target
  (Variables|Default|SetPlayerTarget Target)
  (Variables|Default|SetIsCombat true)
  (Actor|Tick|SetActorTickEnabled true)
  (Variables|Default|SetStart%20Combat%20Location (Transformation|GetActorLocation))
  (CallFunction|FMovementState "NewEnumerator2")
  (CallFunction|CheckforTaunt))

(event EventTick
  (params (DeltaSeconds :type Float%20%28single-precision%29))
  ;[1 1 1] Set Player Target
  (if (Variables|Default|GetIsCombat)
    (Variables|Default|GetPlayerTarget
      (:then
        (Transformation|SetActorRotation (Math|Rotator|MakeRotator 0.0 0.0 (.yaw (Math|Rotator|FindLookatRotation (Transformation|GetActorLocation) (Transformation|GetActorLocation (Variables|Default|GetPlayerTarget)))))))
      (:else))))

(event EventChasePlayer
  ;[1 1 1] Chase Player
  (if (Variables|Default|GetIsCombat)
    (AI|AIMoveTo self "0, 0, 0" (Variables|Default|GetPlayerTarget) 3.5e+02 true
      (:OnSuccess
        (CallFunction|RunAttacks)))))

(event EventCheckforTaunt
  (bind _taunt_montage (Variables|EnemyInfo|GetTaunt%20Montage))
  (bind _output (CallFunction|FGetMontage _taunt_montage))
  ;[1 1 1] Taunt/Aggro
  (AI|Navigation|StopMovement (Pawn|GetController))
  (if (>= (Transformation|GetDistanceTo self (Variables|Default|GetPlayerTarget)) 1.5e+03)
    (CallFunction|PlayMontage (Variables|Character|GetMesh) _output "None")
    (bind _returnvalue (Animation|GetPlayLength _output))
    (Utilities|FlowControl|Delay _returnvalue)
    (CallFunction|ChasePlayer)
    (else
      (CallFunction|ChasePlayer))))

(event EventClearTarget)

(event EventSetMeleeCollision
  (params (State :type Boolean))
  (bind _melee_sphere (Variables|Default|GetMelee%20Sphere))
  (if State
    (Collision|SetCollisionEnabled _melee_sphere "QueryOnly")
    (else
      (Collision|SetCollisionEnabled _melee_sphere "NoCollision"))))

(fn ConstructionScript
  (|CallParentFunction))

(fn FMovementState
  (params (State :type E_AIMovementState%20Enum :default "NewEnumerator0"))
  (bind _walkspeed (Variables|EnemyInfo|GetWalkSpeed))
  (Variables|/Script/Engine.CharacterMovementComponent|SetMaxWalkSpeed (Variables|Character|GetCharacterMovement) (Utilities|Select :Index State :NewEnumerator0 0.0 :NewEnumerator1 _walkspeed :NewEnumerator2 (* (Variables|EnemyInfo|GetSpeedMultiplier) _walkspeed))))

(fn FPickAttack
  (params (Distance%20To%20Player :type Float%20%28single-precision%29))
  (bind _lightattackmontages (Variables|EnemyInfo|GetLightAttackMontages))
  (bind _output (CallFunction|FGetMontage _lightattackmontages))
  (if (<= Distance%20To%20Player (Variables|EnemyInfo|GetMeleeDistance))
    (CallFunction|PlayMontage (Variables|Character|GetMesh) _output "None")
    (bind _returnvalue (Animation|GetPlayLength _output))
    (return _returnvalue)))

(fn FGetMontage
  (params (Montage :type Array%20of%20Anim%20Montage%20Object%20References))
  (return (Utilities|Array|Get(acopy) Montage (Math|Random|RandomIntegerinRange 0 (- (Utilities|Array|Length Montage) 1)))))
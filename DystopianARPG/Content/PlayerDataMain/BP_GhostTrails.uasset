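; BP_GhostTrails is a short-lived afterimage actor that mirrors the player character's current pose as a fading ghost.
; On BeginPlay it gets the player's BP_MainClass, gives each Ghost material slot a dynamic MI_GhostTrail instance and copies the pose from the player's mesh.
; An Opacity timeline drives the Opacity parameter on those instances, then destroys the actor when it finishes.
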(event Custom|GhostTrails
  (for _array_element (Rendering|Material|GetMaterials (Variables|Default|GetGhost))
    (bind _returnvalue (Rendering|Material|CreateDynamicMaterialInstance "/Game/PlayerDataMain/MI_GhostTrail.MI_GhostTrail" "None" :!class /Script/Engine.KismetMaterialLibrary))
    (bind _returnvalue_2 (Utilities|Array|Add (Variables|Default|GetDynamicMats) _returnvalue))
    (Rendering|Material|SetMaterial (Variables|Default|GetGhost) _returnvalue_2 _returnvalue)
    (Class|PoseableMeshComponent|CopyPosefromSkeletalComponent (Variables|Default|GetGhost) (Variables|/Script/Engine.Character|GetMesh (Variables|Default|GetPlayerCharacterRef)))
    (Components|Timeline|PlayfromStart (Variables|Colors|GetOpacity))))

(event EventBeginPlay
  (bind _asbp_main_class (Utilities|Casting|CastToBP_MainClass (Game|Player|GetPlayerPawn 0)))
  (Variables|Default|SetPlayerCharacterRef _asbp_main_class)
  (CallFunction|GhostTrails))

(fn ConstructionScript)
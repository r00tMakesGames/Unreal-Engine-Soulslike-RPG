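; Player controller Blueprint that manages the local player's HUD and death screen.
; Shortly after BeginPlay it creates W_PlayerUI, only for the local controller, and adds it to the viewport.
; UpdateHealthUI and DeathScreenUI forward to client-named events, which update the health bar or clear all widgets and show W_DeathScreen.
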(event Custom|Client_UpdateHealthUI
  (params (Health :type Float%20%28single-precision%29))
  (Default|UpdateHealthBar (Variables|Default|GetPlayer%20UI) Health))

(event Custom|client_createdeathscreen
  (Viewport|RemoveAllWidgets)
  (bind _returnvalue (UserInterface|CreateWidget "/Game/UI/W_DeathScreen.W_DeathScreen_C"))
  (UserInterface|Viewport|AddtoViewport _returnvalue 0))

(event EventBeginPlay
  (Utilities|FlowControl|Delay 0.2)
  (if (Pawn|IsLocalPlayerController)
    (bind _returnvalue (UserInterface|CreateWidget "/Game/UI/W_PlayerUI.W_PlayerUI_C"))
    (bind _output_get (Variables|Default|SetPlayer%20UI _returnvalue))
    (UserInterface|Viewport|AddtoViewport _output_get 0)))

(event EventTick
  (params (DeltaSeconds :type Float%20%28single-precision%29)))

(event EventUpdateHealthUI
  (params (NewHealth :type Float%20%28single-precision%29))
  (CallFunction|ClientUpdateHealthUI NewHealth))

(event EventDeathScreenUI
  (CallFunction|ClientCreatedeathscreen))

(fn ConstructionScript)